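; BP_TestDude is a test character that responds to recognized verb-and-object commands through TT command, interactor, mood, inventory and crafter components.
; Non-GoTo commands queue a move to the named visible target.
; High-fives are gated by mood checks on both giving and receiving, and Store transfers a named item into another actor's inventory.
; Hug is debug logic that prints missing campfire ingredients and spawns sticks; PickUp and unknown commands only print feedback.
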(event OnStore(TTCommandListener)
  (params (verb :type FVerbEnum%20Enum :default "CE_Unknown") (object1 :type String) (object2 :type String))
  ;[1 1 1] Check if inventory exists
  (bind _returnvalue (Class|TTInventoryComponent|GetItembyName (Variables|Default|GetTTInventory) (Utilities|String|StringToName object1)))
  (Utilities|IsValid _returnvalue
    (:Is%20Valid
      (bind _returnvalue_2 (Class|TTInteractorComponent|GetClosestInteractable (Variables|Default|GetTTInteractor) (Utilities|String|StringToName object2)))
      (Utilities|IsValid (Actor|GetComponentbyClass (Components|GetOwner _returnvalue_2) "/Script/GP2_Team3.TTInventoryComponent")
        (:Is%20Valid
          (Class|TTInventoryComponent|RemoveItemfromInventory (Variables|Default|GetTTInventory) _returnvalue)
          (Class|TTInventoryComponent|AddtoInventory (Actor|GetComponentbyClass (Components|GetOwner _returnvalue_2) "/Script/GP2_Team3.TTInventoryComponent") _returnvalue))))))

(event OnHighFive(TTCommandListener)
  (params (object :type String))
  (bind _returnvalue (Class|TTInteractorComponent|GetClosestVisible (Variables|Default|GetTTInteractor) (Utilities|String|StringToName object)))
  (Utilities|IsValid _returnvalue
    (:Is%20Valid
      (Utilities|IsValid (Actor|GetComponentbyClass (Components|GetOwner _returnvalue) "/Script/GP2_Team3.TTMoodComponent")
        (:Is%20Valid
          (bind _returnvalue_2 (Class|TTMoodComponent|DoIWantThis (Variables|Default|GetTTMood_0) "Highfive" (Actor|GetComponentbyClass (Components|GetOwner _returnvalue) "/Script/GP2_Team3.TTMoodComponent")))
          (if _returnvalue_2
            (Class|TTInteractableComponent|Highfive _returnvalue (Variables|Default|GetTTInteractor) :!label _label)
            (else
              (Development|PrintString "No I dont want to"))))
        (:Is%20Not%20Valid
          (goto _label))))))

(event OngetHighfived(TTInteractable)
  (params (interactor :type TT%20Interactor%20Component%20Object%20Reference))
  (bind _returnvalue (Components|GetOwner interactor))
  (bind _returnvalue_2 (Actor|GetComponentbyClass _returnvalue "/Script/GP2_Team3.TTMoodComponent"))
  (bind _asbp_cool_dude (Utilities|Casting|CastToBP_CoolDude _returnvalue))
  (Utilities|IsValid _returnvalue_2
    (:Is%20Valid
      (bind _returnvalue_3 (Class|TTMoodComponent|DoILikeThis (Variables|Default|GetTTMood_0) "Hug" _returnvalue_2 false))
      (if _returnvalue_3
        (Development|PrintString (Utilities|String|Append (Variables|/Game/Blueprints/Character/BP_CoolDude.BP_CoolDude_C|GetName _asbp_cool_dude) " highfived " (Variables|Default|GetName)) :!label _label)
        (else
          (Development|PrintString (Utilities|String|Append (Variables|/Game/Blueprints/Character/BP_CoolDude.BP_CoolDude_C|GetName _asbp_cool_dude) " Rejected  " (Variables|Default|GetName) "'s" " highfive")))))
    (:Is%20Not%20Valid
      (goto _label))))

(event OnHug(TTCommandListener)
  (params (object :type String))
  (Development|PrintString "Hug!!")
  (bind _returnvalue (Class|TTCrafterComponent|WhatAmIMissing (Variables|Default|GetTTCrafter) (Variables|Default|GetTTInventory) "campfire"))
  (for _array_element _returnvalue
    (Development|PrintString (Utilities|String|Append "You need " (Utilities|String|ToString(Integer) (.amount _array_element)) " more " (Utilities|String|ToString(Name) (.dispayname _array_element)) "'s"))
    (bind _returnvalue_2 (Game|SpawnActorfromClass "/Game/Blueprints/Actors/Items/Resources/BP_Stick.BP_Stick_C" (Transformation|GetActorTransform) "Undefined" 0 0)))
  (bind _returnvalue_3 (Class|TTInventoryComponent|AddtoInventory (Variables|Default|GetTTInventory) (Actor|GetComponentbyClass _returnvalue_2 "/Script/GP2_Team3.TTStoreableComponent")))
  (Development|PrintString "Added stick!!" _returnvalue_3))

(event OnPickUp(TTCommandListener)
  (params (verb :type FVerbEnum%20Enum :default "CE_Unknown") (object1 :type String) (object2 :type String))
  ;[1 1 1] BRUNO LOOK HERE!!!!!!!!!!!!!!!!!!!
  ;;[1 1 1] Pick Up Verb was recognized
  (if (Utilities|Enum|NotEqual(Enum) object1 "")
    ;;;[1 1 1] Object was recognized
    (Development|PrintString (Utilities|String|Append "Ok, picking up " object1))
    (else
      (Development|PrintString "What do you want me to pick up?") ; No object was recognized
    )))

(event OnCommand(TTCommandListener)
  (params (command :type FVerbEnum%20Enum :default "CE_Unknown") (object :type String))
  (if (Utilities|Enum|NotEqual(Enum) command "CE_GoTo")
    (bind _returnvalue (Class|TTInteractorComponent|GetClosestVisible (Variables|Default|GetTTInteractor) (Utilities|String|StringToName object)))
    (Class|TTCommandListenerComponent|AddMoveCommand (Variables|Default|GetTTCommandListener) (Transformation|GetActorLocation (Components|GetOwner _returnvalue)))))

(event OnUnknownCommand(TTCommandListener)
  ;[1 1 1] BRUNO LOOK HERE!!!!!!!!!!!!!!!!!!!
  ;;[1 1 1] No verb (like "pick up") was recognized
  (Development|PrintString "Sorry, didn't quite get that."))

(event EventBeginPlay
  (|CallParentFunction) ; This node is disabled and will not be called.\nDrag off pins to build functionality.
)

(event Collision|EventActorBeginOverlap
  (params (OtherActor :type Actor%20Object%20Reference)))

(event EventTick
  (params (DeltaSeconds :type Float%20%28single-precision%29))
  (|CallParentFunction DeltaSeconds) ; This node is disabled and will not be called.\nDrag off pins to build functionality.
)

(fn ConstructionScript
  (|CallParentFunction))