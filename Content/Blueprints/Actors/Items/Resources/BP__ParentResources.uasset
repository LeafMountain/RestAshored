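; Base resource item actor that characters can detect, pick up and drop, showing a WBP_Items name label while overlapped.
; Mesh overlaps register its TTInteractable with the TTCharacter, toggle the label and play a sound.
; Pickup hides the label and disables collision; drop plays a montage on BP_CoolDude, whose notify detaches the item and restores physics and collision.
; Use and eat only pop a random message balloon over BP_CoolDude.
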(event OnComponentBeginOverlap(StaticMesh)
  (params (OverlappedComponent :type Primitive%20Component%20Object%20Reference) (OtherActor :type Actor%20Object%20Reference) (OtherComp :type Primitive%20Component%20Object%20Reference) (OtherBodyIndex :type Integer) (bFromSweep :type Boolean) (SweepResult :type Hit%20Result%20Structure%20%28by%20ref%29))
  (bind _asttcharacter (Utilities|Casting|CastToTTCharacter OtherActor))
  (Class|TTCharacter|AddVisibleInteractable _asttcharacter (Variables|Default|GetTTInteractable))
  (Rendering|SetVisibility (Variables|Default|GetWidget) true false)
  ;[1 0 0.8412] Comment
  (Audio|PlaySound2D "/Game/Audio/PlaceHolders/InteractablesOn_v01_Cue.InteractablesOn_v01_Cue" 1.0 1.0 0.0 0 0))

(event OnComponentEndOverlap(StaticMesh)
  (params (OverlappedComponent :type Primitive%20Component%20Object%20Reference) (OtherActor :type Actor%20Object%20Reference) (OtherComp :type Primitive%20Component%20Object%20Reference) (OtherBodyIndex :type Integer))
  (bind _asttcharacter (Utilities|Casting|CastToTTCharacter OtherActor))
  (Class|TTCharacter|RemoveVisibleInteractable _asttcharacter (Variables|Default|GetTTInteractable))
  (Rendering|SetVisibility (Variables|Default|GetWidget) false false)
  ;[1 0 0.8412] Comment
  (Audio|PlaySound2D "/Game/Audio/PlaceHolders/InteractablesOn_v01_Cue.InteractablesOn_v01_Cue" 1.0 1.0 0.0 0 0))

(event OnPickup(TTInteractable)
  (params (interactor :type TT%20Interactor%20Component%20Object%20Reference) (inventory :type TT%20Inventory%20Component%20Object%20Reference))
  (Rendering|SetVisibility (Variables|Default|GetWidget) false false)
  (Collision|SetCollisionEnabled (Variables|Default|GetStaticMesh) "NoCollision"))

(event OnDrop(TTInteractable)
  (params (interactor :type TT%20Interactor%20Component%20Object%20Reference))
  (bind _asbp_cool_dude (Utilities|Casting|CastToBP_CoolDude (Components|GetOwner interactor)))
  (Animation|Montage|PlayMontage (Variables|/Script/Engine.Character|GetMesh _asbp_cool_dude) "/Game/3D/Animation/Human/AM_Drop.AM_Drop"
    (:OnNotifyBegin
      (Transformation|DetachFromActor "KeepWorld" "KeepWorld" "KeepWorld")
      (Physics|SetSimulatePhysics (Variables|Default|GetStaticMesh) true)
      (Collision|SetCollisionEnabled (Variables|Default|GetStaticMesh) "QueryAndPhysics")
      ;[1 0 0.7985] Comment
      (Audio|PlaySound2D (Variables|Default|GetOnDrop) 1.0 1.0 0.0 0 0))))

(event OnUse(TTInteractable)
  (params (equiper :type TT%20Equiper%20Component%20Object%20Reference) (equipment :type Actor%20Object%20Reference))
  (bind _asbp_cool_dude (Utilities|Casting|CastToBP_CoolDude (Components|GetOwner equiper)))
  (bind (_output _returnvalue) (CallFunction|GetRandomTextMessagefromArray (Variables|Default|GetOnUse)))
  (Default|PopUPBaloon _asbp_cool_dude _output 2.5 _returnvalue))

(event OnEat(TTInteractable)
  (params (interactor :type TT%20Interactor%20Component%20Object%20Reference))
  (bind _asbp_cool_dude (Utilities|Casting|CastToBP_CoolDude (Components|GetOwner interactor)))
  (bind (_output _returnvalue) (CallFunction|GetRandomTextMessagefromArray (Variables|Default|GetOnEat)))
  (Default|PopUPBaloon _asbp_cool_dude _output 2.5 _returnvalue))

(event EventBeginPlay
  (bind _returnvalue (UserInterface|CreateWidget "/Game/Blueprints/UI/WBP_Items.WBP_Items_C" (Game|GetPlayerController 0)))
  (Variables|/Game/Blueprints/UI/WBP_Items.WBP_Items_C|SetItemText _returnvalue (Utilities|Text|ToText(Name) (Variables|Default|GetName)))
  (UserInterface|SetWidget (Variables|Default|GetWidget) _returnvalue))

(fn ConstructionScript)