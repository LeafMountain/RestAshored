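; BP_Storage is an interactable storage actor that stores and hands back equipment through a TTInventory.
; Using it with storeable equipment in hand makes the user drop the item, adds it to the inventory and hides its mesh.
; Using it empty-handed removes the item at index zero, then equips and reveals it if it is equipable.
; A debug loop printing inventory contents is left unconnected.
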(event OnUse(TTInteractable)
  (params (equiper :type TT%20Equiper%20Component%20Object%20Reference) (equipment :type Actor%20Object%20Reference))
  (bind _ttinventory (Variables|Default|GetTTInventory))
  (bind _rootcomponent (Variables|/Script/Engine.Actor|GetRootComponent equipment))
  (bind _returnvalue (Components|GetOwner _rootcomponent))
  (bind _returnvalue_2 (Actor|GetComponentbyClass _returnvalue "/Script/GP2_Team3.TTStoreableComponent"))
  (Utilities|IsValid equipment
    (:Is%20Valid
      (Utilities|IsValid _returnvalue_2
        (:Is%20Valid
          (Class|TTEquiperComponent|DropEquipment equiper)
          (Class|TTInventoryComponent|AddtoInventory (Variables|Default|GetTTInventory) _returnvalue_2)
          (bind _returnvalue_3 (Class|TTInventoryComponent|GetInventoryArray (Variables|Default|GetTTInventory)))
          (Rendering|SetVisibility (Actor|GetComponentbyClass _returnvalue "/Script/Engine.MeshComponent") false false))))
    (:Is%20Not%20Valid
      ;[1 1 1] If nothing equipped
      (bind _returnvalue_4 (Class|TTInventoryComponent|GetItem _ttinventory))
      (Utilities|IsValid _returnvalue_4
        (:Is%20Valid
          (Class|TTInventoryComponent|RemoveItemfromInventory _ttinventory _returnvalue_4)
          (Utilities|IsValid (Actor|GetComponentbyClass (Components|GetOwner _returnvalue_4) "/Script/GP2_Team3.TTEquipableComponent")
            (:Is%20Valid
              (Class|TTEquiperComponent|Equip equiper (Actor|GetComponentbyClass (Components|GetOwner _returnvalue_4) "/Script/GP2_Team3.TTEquipableComponent"))
              (Rendering|SetVisibility (Actor|GetComponentbyClass (Components|GetOwner _returnvalue_4) "/Script/Engine.MeshComponent") true false))))))))

(event EventBeginPlay)

(event Collision|EventActorBeginOverlap
  (params (OtherActor :type Actor%20Object%20Reference)))

(event EventTick
  (params (DeltaSeconds :type Float%20%28single-precision%29)))

(fn ConstructionScript)