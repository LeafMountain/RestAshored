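; BP_BridgeTree is a harvestable tree item whose own event overrides are currently empty, with its earlier logic left disconnected.
; The unreachable use logic checks the equipped tool's class, advances harvest progress and grants resources to the user's inventory, or stops interaction.
; The unreachable depletion logic drops the mesh with physics, removes interaction, destroys both meshes after a delay and notifies the player controller of gathered wood.
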(event EventOnResourceDepleted)

(event EventOnUse
  (params (Equiper :type TT%20Equiper%20Component%20Object%20Reference) (Equipment :type Actor%20Object%20Reference) (DeltaTime :type Float%20%28single-precision%29)))

(event EventOnHarvested)

(fn ConstructionScript
  (|CallParentFunction))