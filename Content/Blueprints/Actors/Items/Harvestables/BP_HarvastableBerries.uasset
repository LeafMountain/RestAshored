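; BP_HarvastableBerries is a harvestable berry item that gives resources when used and respawns after depletion.
; OnUse advances the TTHarvestable progression with delta time, then calls GetResource with the actor's transform and the inventory component of the Equiper's owner.
; On depletion it runs the parent logic, hides the static mesh, then shows it again after the TimerRespawnBerries delay.
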(event EventOnResourceDepleted
  (|CallParentFunction)
  (Rendering|SetVisibility (Variables|Default|GetStaticMesh1) false false)
  (Utilities|FlowControl|Delay (Variables|Default|GetTimerRespawnBerries))
  (Rendering|SetVisibility (Variables|Default|GetStaticMesh1) true false))

(event EventOnUse
  (params (Equiper :type TT%20Equiper%20Component%20Object%20Reference) (Equipment :type Actor%20Object%20Reference) (DeltaTime :type Float%20%28single-precision%29))
  (Class|TTHarvestable|UpdateProgression (Variables|Default|GetTTHarvestable) DeltaTime)
  (CallFunction|GetResource (Transformation|GetActorTransform) (Actor|GetComponentbyClass (Components|GetOwner Equiper) "/Script/GP2_Team3.TTInventoryComponent")))

(fn ConstructionScript
  (|CallParentFunction))