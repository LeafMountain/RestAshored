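; Harvestable fish actor that yields a resource when used with a specific class of equipment and respawns after being depleted.
; On use with matching equipment, it advances the TTHarvestable progression and calls GetResource with the inventory component of the equiper's owner.
; On depletion, it hides the mesh and disables its collision, then restores both after the TimerRespawnFish delay.
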(event EventBeginPlay
  (|CallParentFunction))

(event Collision|EventActorBeginOverlap
  (params (OtherActor :type Actor%20Object%20Reference))
  (|CallParentFunction OtherActor) ; This node is disabled and will not be called.\nDrag off pins to build functionality.
)

(event EventOnHarvested)

(event EventOnUse
  (params (Equiper :type TT%20Equiper%20Component%20Object%20Reference) (Equipment :type Actor%20Object%20Reference) (DeltaTime :type Float%20%28single-precision%29))
  (Utilities|IsValid Equipment
    (:Is%20Valid
      (if (== (Utilities|GetClass Equipment) (Variables|Default|GetActorReference))
        (Class|TTHarvestable|UpdateProgression (Variables|Default|GetTTHarvestable) DeltaTime)
        (CallFunction|GetResource (Transformation|GetActorTransform) (Actor|GetComponentbyClass (Components|GetOwner Equiper) "/Script/GP2_Team3.TTInventoryComponent"))))))

(event EventOnResourceDepleted
  (|CallParentFunction)
  (Rendering|SetVisibility (Variables|Default|GetStaticMesh) false false)
  (Collision|SetCollisionEnabled (Variables|Default|GetStaticMesh) "NoCollision")
  (Utilities|FlowControl|Delay (Variables|Default|GetTimerRespawnFish))
  (Rendering|SetVisibility (Variables|Default|GetStaticMesh) true false)
  (Collision|SetCollisionEnabled (Variables|Default|GetStaticMesh) "QueryAndPhysics"))

(event EventTick
  (params (DeltaSeconds :type Float%20%28single-precision%29))
  (|CallParentFunction DeltaSeconds) ; This node is disabled and will not be called.\nDrag off pins to build functionality.
)

(fn ConstructionScript
  (|CallParentFunction))