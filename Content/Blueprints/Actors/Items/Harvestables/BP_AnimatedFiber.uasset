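; Harvestable fiber actor that animates its static mesh with a small randomized rotation.
; On BeginPlay it picks two random angles within a few degrees of zero, using the first for both roll and yaw and the second for pitch.
; A timeline then drives a rotator lerp from the default rotation toward that target, updating the mesh's relative rotation each update.
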(event EventBeginPlay
  (Variables|Default|SetRandomFloat_01 (Math|Random|RandomFloatinRange -5.0 5.0))
  (Variables|Default|SetRandomFloat_02 (Math|Random|RandomFloatinRange -5.0 5.0))
  (bind _newtrack_0 (Timeline|Timeline_0 PlayFromStart)
    (:Update
      (Transformation|SetRelativeRotation (Variables|Default|GetStaticMesh) (Math|Rotator|Lerp(Rotator) "0, 0, 0" (Math|Rotator|MakeRotator (Variables|Default|GetRandomFloat_01) (Variables|Default|GetRandomFloat_02) (Variables|Default|GetRandomFloat_01)) _newtrack_0) false false))))

(fn ConstructionScript)