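; Animated fish actor, filed under harvestable items, that moves its skeletal mesh around within the actor.
; On BeginPlay it picks two small random offsets, then starts a timeline that lerps the mesh's relative location between two points built from them.
; Each update also sets only the mesh's yaw, from a look-at toward its scaled forward vector.
; A world-rotation lerp node is left unconnected.
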(event EventBeginPlay
  (bind _skeletalmesh (Variables|Default|GetSkeletalMesh))
  (Variables|Default|SetRandomFloat_01 (Math|Random|RandomFloatinRange -2e+01 2e+01))
  (Variables|Default|SetRandomFloat_02 (Math|Random|RandomFloatinRange -2e+01 2e+01))
  (bind _newtrack_0 (Timeline|Timeline_0 PlayFromStart)
    (:Update
      (Transformation|SetRelativeLocation _skeletalmesh (Math|Vector|Lerp(Vector) (Math|Vector|MakeVector (Variables|Default|GetRandomFloat_01) (Variables|Default|GetRandomFloat_02) 0.0) (Math|Vector|MakeVector 0.0 (Variables|Default|GetRandomFloat_01) (Variables|Default|GetRandomFloat_02)) _newtrack_0) false false)
      (Transformation|SetRelativeRotation _skeletalmesh (Math|Rotator|MakeRotator 0.0 0.0 (.yaw (Math|Rotator|FindLookatRotation (Variables|/Script/Engine.SceneComponent|GetRelativeLocation _skeletalmesh) (* (Math|Vector|GetForwardVector _skeletalmesh) 1e+03)))) false false))))

(fn ConstructionScript)