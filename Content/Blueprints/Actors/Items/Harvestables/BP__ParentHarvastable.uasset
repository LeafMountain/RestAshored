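; Base Blueprint for harvestable world items, exposing OnUse and OnHarvested hooks for children.
; Overlapping characters register its interactable and see a name widget.
; GetResource harvests through TTHarvestable, spawns the item and adds it to an inventory; depletion shows a player speech balloon, stops their event and starts a respawn timer restoring one unit.
; The construction script can scatter randomly scaled child actors as procedural visuals.
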(event OnUse(TTInteractable)
  (params (equiper :type TT%20Equiper%20Component%20Object%20Reference) (equipment :type Actor%20Object%20Reference))
  (CallFunction|OnUse equiper equipment 0.0))

(event OnBeenHarvested(TTHarvestable)
  (CallFunction|OnHarvested)
  ;[1 0 0.654] Comment
  (bind _onharvesting (Variables|Default|GetOnHarvesting)
    (:then
      (Audio|PlaySound2D _onharvesting 1.0 1.0 0.0 0 0))
    (:else)))

(event OnResourceDepleted(TTHarvestable)
  (CallFunction|OnResourceDepleted)
  ;[0.04892 1 0] Comment
  (bind _asbp_cool_dude (Utilities|Casting|CastToBP_CoolDude (Components|GetOwner (stale OnUseTick(TTInteractable) _output_get))))
  (bind (_output _returnvalue) (CallFunction|GetRandomTextMessagefromArray (Variables|Default|GetOnUseText)))
  (Default|PopUPBaloon _asbp_cool_dude _output 2.5 _returnvalue)
  ;[1 0 0.654] Comment
  (bind _onresourcedeplete (Variables|Default|GetOnResourceDeplete)
    (:then
      (Audio|PlaySound2D _onresourcedeplete 1.0 1.0 0.0 0 0))
    (:else)))

(event OnUseTick(TTInteractable)
  (params (equiper :type TT%20Equiper%20Component%20Object%20Reference) (equipment :type Actor%20Object%20Reference) (DeltaTime :type Float%20%28single-precision%29))
  (CallFunction|OnUse equiper equipment DeltaTime)
  (bind _output_get (Variables|Default|SetEquiper equiper)))

(event OnComponentBeginOverlap(StaticMesh)
  (params (OverlappedComponent :type Primitive%20Component%20Object%20Reference) (OtherActor :type Actor%20Object%20Reference) (OtherComp :type Primitive%20Component%20Object%20Reference) (OtherBodyIndex :type Integer) (bFromSweep :type Boolean) (SweepResult :type Hit%20Result%20Structure%20%28by%20ref%29))
  (bind _asttcharacter (Utilities|Casting|CastToTTCharacter OtherActor))
  (Class|TTCharacter|AddVisibleInteractable _asttcharacter (Variables|Default|GetTTInteractable))
  (Rendering|SetVisibility (Variables|Default|GetWidget) true false)
  (Audio|PlaySound2D "/Game/Audio/PlaceHolders/InteractablesOn_v01_Cue.InteractablesOn_v01_Cue" 1.0 1.0 0.0 0 0))

(event OnComponentEndOverlap(StaticMesh)
  (params (OverlappedComponent :type Primitive%20Component%20Object%20Reference) (OtherActor :type Actor%20Object%20Reference) (OtherComp :type Primitive%20Component%20Object%20Reference) (OtherBodyIndex :type Integer))
  (bind _asttcharacter (Utilities|Casting|CastToTTCharacter OtherActor))
  (Class|TTCharacter|RemoveVisibleInteractable _asttcharacter (Variables|Default|GetTTInteractable))
  (Rendering|SetVisibility (Variables|Default|GetWidget) false false)
  (Audio|PlaySound2D "/Game/Audio/PlaceHolders/InteractablesOn_v01_Cue.InteractablesOn_v01_Cue" 1.0 1.0 0.0 0 0))

(event Custom|FitSurface
  (for _array_element (Variables|Default|GetContentArray)
    (bind _outhit (Collision|LineTraceByChannel (Transformation|GetWorldLocation _array_element) (- (Transformation|GetWorldLocation _array_element) "0, 0,1000.000000") "TraceTypeQuery1" true 0 "None"))
    (Transformation|SetWorldLocationAndRotation _array_element (+ (.ImpactPoint (Collision|BreakHitResult _outhit)) "0, 0,5.000000") (Math|Rotator|FindLookatRotation (.ImpactNormal (Collision|BreakHitResult _outhit)) (.Normal (Collision|BreakHitResult _outhit))) false false)))

(event Custom|On%20Use
  (params (Equiper :type TT%20Equiper%20Component%20Object%20Reference) (Equipment :type Actor%20Object%20Reference) (DeltaTime :type Float%20%28single-precision%29)))

(event Custom|On%20Resource%20Depleted
  (bind _asbp_cool_dude (Utilities|Casting|CastToBP_CoolDude (Components|GetOwner (Variables|Default|GetEquiper))))
  (Default|StopEvent _asbp_cool_dude)
  (Rendering|SetVisibility (Variables|Default|GetWidget) false false)
  (Utilities|Time|SetTimerbyEvent (delegate Custom|Timer) (Variables|Default|GetRespawnTime)))

(event Custom|On%20Harvested)

(event Custom|Timer
  (CallFunction|RespawnStuff))

(event Custom|RespawnStuff
  (Variables|/Script/GP2_Team3.TTHarvestable|SetCurrentAmount (Variables|Default|GetTTHarvestable) 1))

(event EventBeginPlay
  (bind _returnvalue (UserInterface|CreateWidget "/Game/Blueprints/UI/WBP_Items.WBP_Items_C" (Game|GetPlayerController 0)))
  (Variables|/Game/Blueprints/UI/WBP_Items.WBP_Items_C|SetItemText _returnvalue (Utilities|Text|ToText(Name) (Variables|Default|GetName)))
  (UserInterface|SetWidget (Variables|Default|GetWidget) _returnvalue))

(fn ConstructionScript
  (bind _staticmesh (Variables|Default|GetStaticMesh))
  (Components|StaticMesh|SetStaticMesh _staticmesh (Variables|Default|GetContentMesh))
  (if (Variables|Default|GetProceduralContent?)
    (Rendering|SetVisibility _staticmesh false false)
    (Utilities|Array|Clear (Variables|Default|GetClassContentArray))
    (for _index (range 0 (Variables|Default|GetNumberOfAssets))
      (bind _returnvalue (AddComponent|AddChildActorComponent false (Math|Transform|MakeTransform (Math|Vector|MakeVector (* (Variables|Default|GetDistance) (Math|Random|RandomFloatinRange -3.0 3.0)) (* (Variables|Default|GetDistance) (Math|Random|RandomFloatinRange -3.0 3.0)) 0.0) "0, 0, 0" (Math|Conversions|ToVector(Float) (* 1.0 (Math|Random|RandomFloatinRange 1.0 (Variables|Default|GetScaleRandomness)))))))
      (ChildActorComponent|SetChildActorClass _returnvalue (Variables|Default|GetVisualClass))
      (Utilities|Array|Add (Variables|Default|GetClassContentArray) _returnvalue))))

(fn GetResource
  (params (SpawnTransform :type Transform) (NewParam1 :type TT%20Inventory%20Component%20Object%20Reference))
  (bind _returnvalue (Class|TTHarvestable|IsAvailableforHarvest (Variables|Default|GetTTHarvestable)))
  (if _returnvalue
    (bind _returnvalue_2 (Class|TTHarvestable|Harvest (Variables|Default|GetTTHarvestable)))
    (Utilities|IsValid _returnvalue_2
      (:Is%20Valid
        (bind _returnvalue_3 (Game|SpawnActorfromClass (Utilities|GetClass _returnvalue_2) SpawnTransform "Undefined" 0 0))
        (Utilities|IsValid (Actor|GetComponentbyClass _returnvalue_3 "/Script/GP2_Team3.TTStoreableComponent")
          (:Is%20Valid
            (Utilities|IsValid NewParam1
              (:Is%20Valid
                (bind _returnvalue_4 (Class|TTInventoryComponent|AddtoInventory NewParam1 (Actor|GetComponentbyClass _returnvalue_3 "/Script/GP2_Team3.TTStoreableComponent")))
                (Rendering|SetVisibility (Variables|/Script/Engine.Actor|GetRootComponent _returnvalue_3) (not _returnvalue_4) true)))))))))