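; Harvestable stone actor that a player gathers resources from until it is depleted.
; Picking it up through TTInteractable calls the rock harvest action on BP_CoolDude.
; Each use advances TTHarvestable progression by delta time and passes the stone's transform and the user's inventory component to GetResource.
; On depletion it runs the parent logic, then destroys itself.
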(event OnPickup(TTInteractable)
  (params (interactor :type TT%20Interactor%20Component%20Object%20Reference) (inventory :type TT%20Inventory%20Component%20Object%20Reference))
  (bind _asbp_cool_dude (Utilities|Casting|CastToBP_CoolDude (Components|GetOwner interactor)))
  (Default|CustomHarverst _asbp_cool_dude "rock"))

(event EventOnResourceDepleted
  (|CallParentFunction)
  (Actor|DestroyActor))

(event EventOnHarvested)

(event EventOnUse
  (params (Equiper :type TT%20Equiper%20Component%20Object%20Reference) (Equipment :type Actor%20Object%20Reference) (DeltaTime :type Float%20%28single-precision%29))
  (Class|TTHarvestable|UpdateProgression (Variables|Default|GetTTHarvestable) DeltaTime)
  (CallFunction|GetResource (Transformation|GetActorTransform) (Actor|GetComponentbyClass (Components|GetOwner Equiper) "/Script/GP2_Team3.TTInventoryComponent")))

(fn ConstructionScript
  (|CallParentFunction))