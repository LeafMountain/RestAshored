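; Base actor for tool items that the player character can spot, use, pick up and drop.
; Overlaps register it with TTCharacter as interactable and toggle a name widget.
; Pickup attaches it to BP_CoolDude's right hand on a montage notify; use, pickup and drop play optional sounds and random speech balloons.
; Drop detaches with physics, then after a delay respawns a fresh copy and destroys itself; its drop montage is unwired.
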(event OnUse(TTInteractable)
  (params (equiper :type TT%20Equiper%20Component%20Object%20Reference) (equipment :type Actor%20Object%20Reference))
  ;[1 1 1] Use Logic Goes Here!
  ;;[1 0 0.7954] Comment
  (bind _onuse (Variables|Default|GetOnUse)
    (:then
      (Audio|PlaySound2D _onuse 1.0 1.0 0.0 0 0))
    (:else
      _))
  ;;[0 1 0.009934] Comment
  (bind _asbp_cool_dude (Utilities|Casting|CastToBP_CoolDude (Components|GetOwner equiper)))
  (bind (_output _returnvalue) (CallFunction|GetRandomTextMessagefromArray (Variables|Default|GetOnUseText)))
  (Default|PopUPBaloon _asbp_cool_dude _output 2.5 _returnvalue))

(event OnComponentBeginOverlap(StaticMesh)
  (params (OverlappedComponent :type Primitive%20Component%20Object%20Reference) (OtherActor :type Actor%20Object%20Reference) (OtherComp :type Primitive%20Component%20Object%20Reference) (OtherBodyIndex :type Integer) (bFromSweep :type Boolean) (SweepResult :type Hit%20Result%20Structure%20%28by%20ref%29))
  (bind _asttcharacter (Utilities|Casting|CastToTTCharacter OtherActor))
  (Class|TTCharacter|AddVisibleInteractable _asttcharacter (Variables|Default|GetTTInteractable))
  (Rendering|SetVisibility (Variables|Default|GetWidget) true false)
  ;[1 0 0.5473] Comment
  (Audio|PlaySound2D "/Game/Audio/PlaceHolders/InteractablesOn_v01_Cue.InteractablesOn_v01_Cue" 1.0 1.0 0.0 0 0))

(event OnComponentEndOverlap(StaticMesh)
  (params (OverlappedComponent :type Primitive%20Component%20Object%20Reference) (OtherActor :type Actor%20Object%20Reference) (OtherComp :type Primitive%20Component%20Object%20Reference) (OtherBodyIndex :type Integer))
  (bind _asttcharacter (Utilities|Casting|CastToTTCharacter OtherActor))
  (Class|TTCharacter|RemoveVisibleInteractable _asttcharacter (Variables|Default|GetTTInteractable))
  (Rendering|SetVisibility (Variables|Default|GetWidget) false false)
  ;[1 0 0.5473] Comment
  (Audio|PlaySound2D "/Game/Audio/PlaceHolders/InteractablesOn_v01_Cue.InteractablesOn_v01_Cue" 1.0 1.0 0.0 0 0))

(event OnPickup(TTEquipable)
  (params (equiper :type TT%20Equiper%20Component%20Object%20Reference))
  ;[1 1 1] Pick up and eqiup, attach to socket
  (bind _asbp_cool_dude (Utilities|Casting|CastToBP_CoolDude (Components|GetOwner equiper)))
  (Animation|Montage|PlayMontage (Variables|/Script/Engine.Character|GetMesh _asbp_cool_dude) "/Game/3D/Animation/Human/AM_PickUp.AM_PickUp"
    (:OnNotifyBegin
      (Physics|SetSimulatePhysics (Variables|Default|GetStaticMesh) false)
      (Transformation|AttachComponentToComponent (Variables|/Script/Engine.Character|GetMesh _asbp_cool_dude) (Variables|Default|GetRight%20Hand) "SnapToTarget" "SnapToTarget" "KeepWorld" true)
      (Rendering|SetVisibility (Variables|Default|GetWidget) false false)
      ;;[1 0 0.7954] Comment
      (bind _onpickup (Variables|Default|GetOnPickUp)
        (:then
          (Audio|PlaySound2D _onpickup 1.0 1.0 0.0 0 0))
        (:else
          _))
      ;;[0.02776 1 0] Comment
      (bind (_output _returnvalue) (CallFunction|GetRandomTextMessagefromArray (Variables|Default|GetOnPicked)))
      (Default|PopUPBaloon _asbp_cool_dude _output 2.5 _returnvalue))))

(event OnDrop(TTEquipable)
  (params (equiper :type TT%20Equiper%20Component%20Object%20Reference))
  (bind _staticmesh (Variables|Default|GetStaticMesh))
  ;[1 1 1] Drop and turn on physics, destroy and spawn new item
  (bind _asbp_cool_dude (Utilities|Casting|CastToBP_CoolDude (Components|GetOwner equiper)))
  (Physics|SetSimulatePhysics _staticmesh true)
  (Transformation|DetachFromComponent _staticmesh "KeepWorld" "KeepWorld" "KeepWorld" true)
  (Utilities|FlowControl|Delay 2.0)
  (Rendering|SetVisibility (Variables|Default|GetWidget) true false)
  ;;[1 0 0.6408] Comment
  (bind _ondrop (Variables|Default|GetOnDrop)
    (:then
      (Audio|PlaySound2D _ondrop 1.0 1.0 0.0 0 0))
    (:else
      _))
  ;;[0.08068 1 0] Comment
  (bind (_output _returnvalue) (CallFunction|GetRandomTextMessagefromArray (Variables|Default|GetOnDroped)))
  (Default|PopUPBaloon _asbp_cool_dude _output 2.5 _returnvalue)
  (Game|SpawnActorfromClass (Utilities|GetClass self) (Transformation|GetWorldTransform _staticmesh) "Undefined" 0 0)
  (Actor|DestroyActor))

(event EventBeginPlay
  (bind _returnvalue (UserInterface|CreateWidget "/Game/Blueprints/UI/WBP_Items.WBP_Items_C" (Game|GetPlayerController 0)))
  (Variables|/Game/Blueprints/UI/WBP_Items.WBP_Items_C|SetItemText _returnvalue (Utilities|Text|ToText(Name) (Variables|Default|GetName)))
  (UserInterface|SetWidget (Variables|Default|GetWidget) _returnvalue))

(fn ConstructionScript)