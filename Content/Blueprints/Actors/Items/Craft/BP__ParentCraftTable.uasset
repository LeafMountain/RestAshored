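; Parent Blueprint for craft table actors, built around interactable, inventory and crafter components.
; Using the table currently only prints a "Move to Bench" debug message, and the done-crafting event is empty.
; Disconnected draft logic gathers the owners of inventory items, passes them to the crafter and spawns the crafted class at a placeholder location.
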(event OnDoneCrafting(TTCrafter))

(event OnUse(TTInteractable)
  (params (equiper :type TT%20Equiper%20Component%20Object%20Reference) (equipment :type Actor%20Object%20Reference))
  (Development|PrintString "Move to Bench"))

(fn ConstructionScript)