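; Base actor for built items, which snaps itself to the ground and acts as an interactable for TTCharacter.
; On BeginPlay a downward trace places it at the hit point aligned to the surface normal, creates a WBP_Items name label for its widget and plays an optional build sound.
; Mesh overlaps register or remove the interactable on the character, toggle the label's visibility and play a sound cue.
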(event OnComponentBeginOverlap(StaticMesh)
  (params (OverlappedComponent :type Primitive%20Component%20Object%20Reference) (OtherActor :type Actor%20Object%20Reference) (OtherComp :type Primitive%20Component%20Object%20Reference) (OtherBodyIndex :type Integer) (bFromSweep :type Boolean) (SweepResult :type Hit%20Result%20Structure%20%28by%20ref%29))
  (bind _asttcharacter (Utilities|Casting|CastToTTCharacter OtherActor))
  (Class|TTCharacter|AddVisibleInteractable _asttcharacter (Variables|Default|GetTTInteractable))
  (Rendering|SetVisibility (Variables|Default|GetWidget) true false)
  (Audio|PlaySound2D "/Game/Audio/PlaceHolders/InteractablesOn_v01_Cue.InteractablesOn_v01_Cue" 1.0 1.0 0.0 0 0))

(event OnComponentEndOverlap(StaticMesh)
  (params (OverlappedComponent :type Primitive%20Component%20Object%20Reference) (OtherActor :type Actor%20Object%20Reference) (OtherComp :type Primitive%20Component%20Object%20Reference) (OtherBodyIndex :type Integer))
  (bind _asttcharacter (Utilities|Casting|CastToTTCharacter OtherActor))
  (Class|TTCharacter|RemoveVisibleInteractable _asttcharacter (Variables|Default|GetTTInteractable))
  (Rendering|SetVisibility (Variables|Default|GetWidget) false false)
  (Audio|PlaySound2D "/Game/Audio/PlaceHolders/InteractablesOn_v01_Cue.InteractablesOn_v01_Cue" 1.0 1.0 0.0 0 0))

(event EventBeginPlay
  (bind _defaultsceneroot (Variables|Default|GetDefaultSceneRoot))
  (bind _returnvalue (Transformation|GetWorldLocation _defaultsceneroot))
  (bind _outhit (Collision|LineTraceByChannel _returnvalue (- _returnvalue "0, 0,1000.000000") "TraceTypeQuery1" true 0 "None"))
  (Transformation|SetActorLocationAndRotation (.Location (Collision|BreakHitResult _outhit)) (Math|Rotator|MakeRotfromZ (.Normal (Collision|BreakHitResult _outhit))))
  (bind _returnvalue_2 (UserInterface|CreateWidget "/Game/Blueprints/UI/WBP_Items.WBP_Items_C" (Game|GetPlayerController 0)))
  (Variables|/Game/Blueprints/UI/WBP_Items.WBP_Items_C|SetItemText _returnvalue_2 (Utilities|Text|ToText(Name) (Variables|Default|GetName)))
  (UserInterface|SetWidget (Variables|Default|GetWidget) _returnvalue_2)
  ;[1 0 0.7225] Comment
  (bind _itembuildsound (Variables|Default|GetItemBuildSound)
    (:then
      (Audio|PlaySound2D _itembuildsound 1.0 1.0 0.0 0 0))
    (:else)))

(fn ConstructionScript)