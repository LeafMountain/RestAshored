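; Day and night cycle light actor that rotates over a configurable day length and updates the level's BP_Sky_Sphere sun direction.
; Each Tick derives rotation from a looping timer, then uses actor pitch to choose night or day intensity interpolation.
; A DoOnce, reset at night, advances and prints the day count when day returns and calls NewDay on BP_GameMode.
; Light color blending exists but is unconnected.
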(event EventBeginPlay
  ;[1 1 1] Get sky sphere reference
  (bind _outactors (Actor|GetAllActorsOfClass "/Engine/EngineSky/BP_Sky_Sphere.BP_Sky_Sphere_C"))
  (Variables|Default|SetBP_SkySphere%20Ref (Utilities|Array|Get(acopy) _outactors)))

(event EventTick
  (params (DeltaSeconds :type Float%20%28single-precision%29))
  ;[1 1 1] Day and night cycle
  (bind _output_get (Variables|Default|Settimer (+ DeltaSeconds (Variables|Default|Gettimer))))
  (if (>= _output_get (Variables|Default|GetDayNightLength))
    (Variables|Default|Settimer 0.0))
  (Transformation|SetActorRelativeRotation (Math|Rotator|MakeRotator 0.0 (* (/ (Variables|Default|Gettimer) (Variables|Default|GetDayNightLength)) 3.6e+02) (/ (* (/ (Variables|Default|Gettimer) (Variables|Default|GetDayNightLength)) 3.6e+02) 1e+01)))
  (Default|UpdateSunDirection (Variables|Default|GetBP_SkySphere%20Ref))
  (bind _output_get_2 (Variables|Default|SetNight (Math|Float|InRange(Float) (.pitch (Transformation|GetActorRotation)) 0.0 1e+02)))
  (if _output_get_2
    (Utilities|FlowControl|Sequence
      (:then_1
        ;;[1 0.6304 0] Sets intensity of light
        (CallFunction|NightLightning (* (/ (Variables|Default|Gettimer) (Variables|Default|GetDayNightLength)) 3.6e+02))
        (goto _label Reset)))
    (else
      (CallFunction|DayLightning (* (/ (Variables|Default|Gettimer) (Variables|Default|GetDayNightLength)) 3.6e+02))
      ;;[0 1 0.5858] Set Day number (Date) and trigger the "New Day" (Weather system) event inside Game mode.
      (Utilities|FlowControl|DoOnce false :!label _label
        (:Completed
          (bind _day (CallFunction|SetDate))
          (Development|PrintString (Utilities|String|Append "Day " (Utilities|String|ToString(Integer) _day)) true true "(R=0.000000,G=1.000000,B=0.649375,A=1.000000)")
          (bind _asbp_game_mode (Utilities|Casting|CastToBP_GameMode (Game|GetGameMode)))
          (Default|NewDay _asbp_game_mode)
          (Utilities|FlowControl|DoOnce false ; enters at Reset
            (:Completed
              (Transformation|SetActorRelativeRotation (Math|Rotator|MakeRotator 0.0 1.8e+02 0.0)))))))))

(fn ConstructionScript)

(fn NightLightning
  (params (Delta :type Float%20%28single-precision%29))
  (bind _returnvalue (/ Delta 64.0))
  (bind _lightcomponent (Variables|Default|GetLightComponent))
  (bind _intensity (Variables|/Script/Engine.LightComponentBase|GetIntensity _lightcomponent))
  (Rendering|Components|Light|SetIntensity _lightcomponent (Math|Interpolation|FInterpTo _intensity (Variables|Default|GetNightIntensityStart) _returnvalue 3.0))
  (Rendering|Components|Light|SetIntensity _lightcomponent (Math|Interpolation|FInterpTo _intensity (Variables|Default|GetNightIntensityTarget) _returnvalue 5.0)))

(fn DayLightning
  (params (Delta :type Float%20%28single-precision%29))
  (bind _returnvalue (/ Delta 64.0))
  (bind _lightcomponent (Variables|Default|GetLightComponent))
  (bind _intensity (Variables|/Script/Engine.LightComponentBase|GetIntensity _lightcomponent))
  (Rendering|Components|Light|SetIntensity _lightcomponent (Math|Interpolation|FInterpTo _intensity (Variables|Default|GetDayIntensityStart) _returnvalue 4.0))
  (Rendering|Components|Light|SetIntensity _lightcomponent (Math|Interpolation|FInterpTo _intensity (Variables|Default|GetDayIntensityTarget) _returnvalue 8.0)))

(fn SetDate
  (bind _output_get (Variables|Default|SetWhat%20Day%20Is%20It? (+ (Variables|Default|GetWhat%20Day%20Is%20It?) 1)))
  (return _output_get))