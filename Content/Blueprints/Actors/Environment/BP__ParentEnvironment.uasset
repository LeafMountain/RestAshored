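; BP__ParentEnvironment is a base environment actor meant to track night state and current weather, with an empty CustomTick event as a hook.
; Its Timer event calls CustomTick, then copies IsNight from the Sun actor and CurrentWeather from the game mode.
; The setup caching the game mode and Bp_DayAndNight actor and starting the one-second looping timer is disconnected, and BeginPlay is empty, so polling never starts here.
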(event Custom|Timer
  (CallFunction|CustomTick)
  (Variables|Default|SetIsNight? (Variables|/Game/Blueprints/Actors/Environment/Bp_DayAndNight.Bp_DayAndNight_C|GetNight (Variables|Default|GetSun)))
  (bind _gm (Variables|Default|GetGM)
    (:then
      (Variables|Default|SetCurrentWeather (Variables|/Game/Blueprints/BP_GameMode.BP_GameMode_C|GetWeatherEnum _gm)))
    (:else)))

(event Custom|CustomTick)

(event EventBeginPlay)

(fn ConstructionScript)