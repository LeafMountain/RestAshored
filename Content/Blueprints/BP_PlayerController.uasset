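; Player controller for a voice-commanded island survival game, handling the HUD, character selection and task progression.
; Push-to-talk on Left Shift passes recognized speech to the game mode's command system.
; Newly selected units drive camera focus and action widgets, added or removed as their available actions change.
; A MultiGate sequences tasks from camera tutorial to boat repair, spawning task actors, new characters and to-do entries.
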(event Custom|OnWordsSpoken
  (params (Text :type Recognised%20Phrases%20Structure))
  (bind _phrases (Utilities|Struct|BreakRecognisedPhrases Text))
  (bind _saying (Variables|Default|GetSaying))
  (if (Variables|Default|GetIsPressedToTalk)
    ;[1 1 1] Send Command To Command Log
    (Utilities|FlowControl|Sequence
      (:then_0
        (bind _returnvalue (Class|TTGameMode|GetCommandSystem (Variables|Default|GetGM)))
        (Class|TTCommandSystem|StringtoCommand _returnvalue (Utilities|String|JoinStringArray _phrases " ")))
      (:then_1
        (for _array_element _phrases
          (if (not (Utilities|Enum|Equal(Enum) _array_element "/s"))
            (if (not (Utilities|Enum|Equal(Enum) _array_element "[SPEECH]"))
              (Utilities|Array|Add _saying _array_element))))
        (Utilities|Array|Clear _saying)))))

(event Custom|WalkingUsing
  ;[1 1 1] Update walk/stop action widget on timer
  (bind _asbp_cool_dude (Utilities|Casting|CastToBP_CoolDude (Variables|Default|GetSelectedCharacter)))
  (Class|WidgetSwitcher|SetActiveWidgetIndex (Variables|/Game/Blueprints/UI/Actions/WBP_Action_Walk.WBP_Action_Walk_C|GetSwitcher (Variables|Default|GetActionWalk)) (select (Variables|/Game/Blueprints/Character/BP_CoolDude.BP_CoolDude_C|GetWalking? _asbp_cool_dude) 1 0)))

(event Custom|TaskComplete
  (Default|TaskDone (Variables|Default|GetToDoListWidget))
  (Default|CallRemoveSubtasks)
  (Audio|PlaySound2D "/Game/Audio/QuestLog/Quest_Complete_01_Cue.Quest_Complete_01_Cue" 1.0 1.0 0.0 0 0))

(event Custom|OnSpeechRecognitionInitialized_Event_1
  ;[1 1 1] On Plugin Initialized
  (Default|Ready (Variables|Default|GetWBP_Loading))
  (Utilities|FlowControl|Delay 1.0)
  (CallFunction|StartGame))

(event Custom|OnRemovedVisible
  (params (actiontype :type ETTAction%20Enum :default "Walk"))
  ;[1 1 1] Remove Children
  (CallFunction|RemoveActionCommand actiontype))

(event Custom|OnNewUnit_Event_0
  (params (unit :type Actor%20Object%20Reference))
  (if (Variables|Default|GetLockCharacters?)
    _
    (else
      (Default|CameraMovetoCharacter (Variables|Default|GetCameraPawn) unit)))
  (bind _asttcharacter (Utilities|Casting|CastToTTCharacter unit))
  (bind _output_get (Variables|Default|SetSelectedCharacter _asttcharacter))
  (bind _asbp_cool_dude (Utilities|Casting|CastToBP_CoolDude _output_get))
  (bind _output_get_2 (Variables|Default|SetSelectedCooldude _asbp_cool_dude))
  (Default|UIBar (Variables|Default|GetWBP_HUDv03) _output_get_2)
  (Widget|Panel|AddChild (Variables|/Game/Blueprints/UI/WBP_BasicUI_v03.WBP_BasicUI_v03_C|GetWalkGoesHere (Variables|Default|GetWBP_HUDv03)) (Variables|Default|GetActionWalk))
  (EventDispatchers|UnbindEventfromOnStopsbeingAvailable (Variables|Default|GetSelectedCharacter) (delegate Custom|OnRemovedVisible))
  (EventDispatchers|UnbindEventfromOnVisibilityUpdate (Variables|Default|GetSelectedCharacter) (delegate Custom|UpdateCommandsUI))
  (EventDispatchers|BindEventtoOnVisibilityUpdate (Variables|Default|GetSelectedCharacter) (delegate Custom|UpdateCommandsUI))
  (EventDispatchers|BindEventtoOnStopsbeingAvailable (Variables|Default|GetSelectedCharacter) (delegate Custom|OnRemovedVisible)))

(event Custom|CheckWalking
  ;[1 1 1] Update walk/stop action widget on timer
  (Utilities|Time|SetTimerbyEvent (delegate Custom|WalkingUsing) 0.5 true))

(event Custom|SendMessage
  (params (Message :type Text))
  ;[1 1 1] Send Command To Command Log
  (Default|AddMessage (Variables|/Game/Blueprints/UI/WBP_BasicUI_v03.WBP_BasicUI_v03_C|GetWBP_Log (Variables|Default|GetWBP_HUDv03)) Message))

(event Custom|UpdateCommandsUI
  ;[1 1 1] Add Children
  (bind _returnvalue (Class|TTCharacter|GetAvailableActions (Variables|Default|GetSelectedCharacter)))
  (for _array_element _returnvalue
    (if (.isnew _array_element)
      (CallFunction|AddActionCommand (.action _array_element)))))

(event Custom|StartGame
  ;[1 1 1] Create To do list widget
  (bind _returnvalue (UserInterface|CreateWidget "/Game/Blueprints/UI/WBP_ToDoList.WBP_ToDoList_C" (Game|GetPlayerController 0)))
  (bind _output_get (Variables|Default|SetToDoListWidget _returnvalue))
  (UserInterface|Viewport|AddtoViewport _output_get 0)
  (CallFunction|RequestNewTask))

(event Custom|RequestNewTask
  (if (> (Variables|Default|GetTasksIndex) 3)
    (Variables|Default|SetLockCharacters? false))
  (Utilities|FlowControl|MultiGate false false (Variables|Default|GetTasksIndex)
    (:Out%200
      (Default|AddTask (Variables|Default|GetToDoListWidget) "Move the camera: W, A, S, D")
      (Game|SpawnActorfromClass "/Game/Blueprints/Tutorial/BP_Task_MoveCamera.BP_Task_MoveCamera_C" (Transformation|GetActorTransform) "Undefined" 0 0)
      (Variables|Default|SetTutorial? true))
    (:Out%201
      (Default|AddTask (Variables|Default|GetToDoListWidget) "Rotate the camera: Right Mouse and Roll")
      (Game|SpawnActorfromClass "/Game/Blueprints/Tutorial/BP_Task_RotateCamera.BP_Task_RotateCamera_C" (Transformation|GetActorTransform) "Undefined" 0 0))
    (:Out%202
      (Default|AddTask (Variables|Default|GetToDoListWidget) "Zoom In and Out scrolling your mouse")
      (Game|SpawnActorfromClass "/Game/Blueprints/Tutorial/BP_Task_Zooming.BP_Task_Zooming_C" (Transformation|GetActorTransform) "Undefined" 0 0))
    (:Out%203
      (Default|AddTask (Variables|Default|GetToDoListWidget) "Get Stella´s attention: Press and Hold Left Shift to talk")
      (Game|SpawnActorfromClass "/Game/Blueprints/Tutorial/BP_Task_CallStella.BP_Task_CallStella_C" (Transformation|GetActorTransform) "Undefined" 0 0)
      (Variables|Default|SetLockCharacters? false))
    (:Out%204
      (Default|AddTask (Variables|Default|GetToDoListWidget) "Walk to the Camp")
      ;[1 1 1] Available Options
      (CallFunction|AddSubTaskTuturial "/Game/Blueprints/UI/TutorialsSubTasks/WBP_AvailableActions.WBP_AvailableActions_C")
      (bind _outactors (Actor|GetAllActorsOfClass "/Script/Engine.Note"))
      (bind _array_element (Utilities|Array|ForEachLoopwithBreak _outactors :!label _label)
        (:LoopBody
          (if (Utilities|Enum|Equal(Enum) (Variables|/Script/Engine.Note|GetText _array_element) "camp")
            (Game|SpawnActorfromClass "/Game/Blueprints/Tutorial/BP_Task_Find_Camp.BP_Task_Find_Camp_C" (Transformation|GetActorTransform _array_element) "Undefined" 0 0)
            (goto _label Break)))
        (:Completed
          (bind _returnvalue (UserInterface|CreateWidget "/Game/Blueprints/UI/WBP_Actions.WBP_Actions_C" (Game|GetPlayerController 0)))
          (Widget|Panel|AddChild (Variables|/Game/Blueprints/UI/WBP_BasicUI_v02.WBP_BasicUI_v02_C|GetAction (Variables|Default|GetWBP_HUD)) _returnvalue))))
    (:Out%205
      (Default|AddTask (Variables|Default|GetToDoListWidget) "Craft an Axe.")
      (Game|SpawnActorfromClass "/Game/Blueprints/Tutorial/BP_Task_CraftAxe.BP_Task_CraftAxe_C" (Transformation|GetActorTransform) "Undefined" 0 0))
    (:Out%206
      (Default|AddTask (Variables|Default|GetToDoListWidget) "Collect Wood")
      (Game|SpawnActorfromClass "/Game/Blueprints/Tutorial/BP_Task_CollectWood.BP_Task_CollectWood_C" (Transformation|GetActorTransform) "Undefined" 0 0))
    (:Out%207
      (Default|AddTask (Variables|Default|GetToDoListWidget) "Get Eddie's Attention by Selecting Him")
      (Game|SpawnActorfromClass "/Game/Blueprints/Tutorial/BP_Task_CallEddie.BP_Task_CallEddie_C" (Transformation|GetActorTransform) "Undefined" 0 0)
      (Game|SpawnActorfromClass "/Game/Blueprints/Character/BP_CoolEddie.BP_CoolEddie_C" (Math|Transform|MakeTransform "1280.000000,1550.000000,500.000000" "0, 0, 0" "1,1,1") "Undefined" 0 0))
    (:Out%208
      (Default|AddTask (Variables|Default|GetToDoListWidget) "Collect Food")
      (Game|SpawnActorfromClass "/Game/Blueprints/Tutorial/BP_task_CollectFood.BP_task_CollectFood_C" (Transformation|GetActorTransform) "Undefined" 0 0))
    (:Out%209
      (Default|AddTask (Variables|Default|GetToDoListWidget) "Get Astrid's Attention by Selecting Her")
      (Game|SpawnActorfromClass "/Game/Blueprints/Tutorial/BP_Task_CallAstrid.BP_Task_CallAstrid_C" (Transformation|GetActorTransform) "Undefined" 0 0)
      (Game|SpawnActorfromClass "/Game/Blueprints/Character/BP_CoolAstrid.BP_CoolAstrid_C" (Math|Transform|MakeTransform "1280.000000,1550.000000,500.000000" "0, 0, 0" "1,1,1") "Undefined" 0 0))
    (:Out%2010
      (Variables|Default|SetTutorial? false)
      (Default|AddTask (Variables|Default|GetToDoListWidget) "Craft a Fishing Rod")
      (Game|SpawnActorfromClass "/Game/Blueprints/Tutorial/BP_Task_CraftFishingRod.BP_Task_CraftFishingRod_C" (Transformation|GetActorTransform) "Undefined" 0 0))
    (:Out%2011
      (Default|AddTask (Variables|Default|GetToDoListWidget) "Catch some fish")
      (Game|SpawnActorfromClass "/Game/Blueprints/Tutorial/BP_Task_CatchFish.BP_Task_CatchFish_C" (Transformation|GetActorTransform) "Undefined" 0 0))
    (:Out%2012
      (Default|AddTask (Variables|Default|GetToDoListWidget) "Find a safe Water Source")
      (Game|SpawnActorfromClass "/Game/Blueprints/Tutorial/BP_Task_FindWater.BP_Task_FindWater_C" (Transformation|GetActorTransform) "Undefined" 0 0))
    (:Out%2013
      (Default|AddTask (Variables|Default|GetToDoListWidget) "Explore the Island")
      (Game|SpawnActorfromClass "/Game/Blueprints/Tutorial/BP_Task_CraftAxe.BP_Task_CraftAxe_C" (Transformation|GetActorTransform) "Undefined" 0 0))
    (:Out%2014
      (Default|AddTask (Variables|Default|GetToDoListWidget) "Repair the Boat and get of the island")
      (Game|SpawnActorfromClass "/Game/Blueprints/Tutorial/BP_TaskBuildBoat.BP_TaskBuildBoat_C" (Transformation|GetActorTransform) "Undefined" 0 0))))

(event EventBeginPlay
  (Utilities|FlowControl|Sequence
    (:then_0
      (bind _returnvalue (CallFunction|InitializePlayerController))
      (bind _returnvalue_2 (UserInterface|CreateWidget "/Game/Blueprints/UI/WBP_BasicUI_v03.WBP_BasicUI_v03_C" (Game|GetPlayerController 0)))
      (bind _output_get (Variables|Default|SetWBP_HUDv03 _returnvalue_2))
      (UserInterface|Viewport|AddtoViewport _output_get 2)
      (EventDispatchers|AssignOnNewUnit _returnvalue (delegate Custom|OnNewUnit_Event_0)))
    (:then_1
      (bind _returnvalue_3 (Game|SpawnActorfromClass "/Script/SpeechRecognition.SpeechRecognitionActor" (Transformation|GetActorTransform) "Undefined" 0 0))
      (bind _output_get_2 (Variables|Default|SetSpeechRecognition _returnvalue_3))
      (EventDispatchers|AssignOnWordsSpoken _output_get_2 (delegate Custom|OnWordsSpoken))
      (EventDispatchers|AssignOnSpeechRecognitionInitialized (Variables|Default|GetSpeechRecognition) (delegate Custom|OnSpeechRecognitionInitialized_Event_1))
      (bind _returnvalue_4 (Class|SpeechRecognitionActor|Init (Variables|Default|GetSpeechRecognition) "VE_English"))
      (if _returnvalue_4
        (Development|PrintString "Voice Recog - Init Success")
        (CallFunction|SetConfig)
        (Class|SpeechRecognitionActor|EnableLanguageModel (Variables|Default|GetSpeechRecognition) "en")))
    (:then_2
      (CallFunction|CreateActionWidgets))
    (:then_3
      (CallFunction|CheckWalking))))

(event EventEndPlay
  (params (EndPlayReason :type EEndPlayReason%20Enum :default "Destroyed"))
  (Class|SpeechRecognitionActor|Shutdown (Variables|Default|GetSpeechRecognition)))

(event Input|KeyboardEvents|LeftShift
  (params (Key :type Key%20Structure))
  ;[1 1 1] Left Shift Input
  (:Pressed
    (Variables|Default|SetIsShiftPressed true)
    (Variables|Default|SetIsPressedToTalk true)
    (Audio|PlaySound2D "/Game/Audio/PlaceHolders/SC_Press_to_Talk_On.SC_Press_to_Talk_On" 1.0 1.0 0.0 0 0)
    (Utilities|Array|Clear (Variables|Default|GetSaying)))
  (:Released
    (Variables|Default|SetIsShiftPressed false)
    (Audio|PlaySound2D "/Game/Audio/PlaceHolders/SC_Press_To_Talk_Off.SC_Press_To_Talk_Off" 1.0 1.0 0.0 0 0)
    (Utilities|FlowControl|RetriggerableDelay 1.0)
    (if (not (Variables|Default|GetIsShiftPressed))
      (Variables|Default|SetIsPressedToTalk false))))

(fn ConstructionScript)

(fn SetConfig
  (bind _speechrecognition (Variables|Default|GetSpeechRecognition))
  (Class|SpeechRecognitionActor|SetConfigParam _speechrecognition "-vad_prespeech" "VE_INTEGER" "10")
  (Class|SpeechRecognitionActor|SetConfigParam _speechrecognition "-vad_postspeech" "VE_INTEGER" "10")
  (Class|SpeechRecognitionActor|SetConfigParam _speechrecognition "-agc" "VE_STRING" "noise")
  (Class|SpeechRecognitionActor|SetConfigParam _speechrecognition "-beam" "VE_FLOAT" "1e-40"))

(fn InitializePlayerController
  (bind _asbp_camera_pawn (Utilities|Casting|CastToBP_CameraPawn (Game|Player|GetPlayerPawn 0)))
  (Variables|Default|SetCameraPawn _asbp_camera_pawn)
  (bind _asbp_game_mode (Utilities|Casting|CastToBP_GameMode (Game|GetGameMode)))
  (bind _output_get (Variables|Default|SetGM _asbp_game_mode))
  (bind _returnvalue (Class|TTGameMode|GetCommandSystem _output_get))
  (bind _outactors (Actor|GetAllActorsOfClass "/Script/Engine.Note"))
  (Variables|Default|SetSpawnLocations _outactors)
  (return _returnvalue))

(fn CreateActionWidgets
  (bind _returnvalue (Game|GetPlayerController 0))
  (bind _returnvalue_2 (UserInterface|CreateWidget "/Game/Blueprints/UI/Actions/WBP_Action_Collect.WBP_Action_Collect_C" _returnvalue))
  (Variables|Default|SetActionCollect _returnvalue_2)
  (bind _returnvalue_3 (UserInterface|CreateWidget "/Game/Blueprints/UI/Actions/WBP_Action_Craft.WBP_Action_Craft_C" _returnvalue))
  (Variables|Default|SetActionCraft _returnvalue_3)
  (bind _returnvalue_4 (UserInterface|CreateWidget "/Game/Blueprints/UI/Actions/WBP_Action_Drop.WBP_Action_Drop_C" _returnvalue))
  (Variables|Default|SetActionDrop _returnvalue_4)
  (bind _returnvalue_5 (UserInterface|CreateWidget "/Game/Blueprints/UI/Actions/WBP_Action_Equip.WBP_Action_Equip_C" _returnvalue))
  (Variables|Default|SetActionEquip _returnvalue_5)
  (bind _returnvalue_6 (UserInterface|CreateWidget "/Game/Blueprints/UI/Actions/WBP_Action_PickUp.WBP_Action_PickUp_C" _returnvalue))
  (Variables|Default|SetActionPickUp _returnvalue_6)
  (bind _returnvalue_7 (UserInterface|CreateWidget "/Game/Blueprints/UI/Actions/WBP_Action_Walk.WBP_Action_Walk_C" _returnvalue))
  (Variables|Default|SetActionWalk _returnvalue_7)
  (bind _returnvalue_8 (UserInterface|CreateWidget "/Game/Blueprints/UI/Actions/WBP_Action_Use.WBP_Action_Use_C" _returnvalue))
  (Variables|Default|SetActionUse _returnvalue_8)
  (bind _returnvalue_9 (UserInterface|CreateWidget "/Game/Blueprints/UI/Actions/WBP_Action_Store.WBP_Action_Store_C" _returnvalue))
  (Variables|Default|SetActionStore _returnvalue_9)
  (bind _returnvalue_10 (UserInterface|CreateWidget "/Game/Blueprints/UI/Actions/WBP_Action_Stop.WBP_Action_Stop_C" _returnvalue))
  (Variables|Default|SetActionStop _returnvalue_10)
  (bind _returnvalue_11 (UserInterface|CreateWidget "/Game/Blueprints/UI/Actions/WBP_Action_Eat.WBP_Action_Eat_C" _returnvalue))
  (Variables|Default|SetActionEat _returnvalue_11))

(fn AddActionCommand
  (params (Selection :type ETTAction%20Enum :default "Walk"))
  (bind _wbp_hudv03 (Variables|Default|GetWBP_HUDv03))
  (bind _actioneat (Variables|Default|GetActionEat))
  (bind _actioncollect (Variables|Default|GetActionCollect))
  (bind _actioncraft (Variables|Default|GetActionCraft))
  (bind _actiondrop (Variables|Default|GetActionDrop))
  (bind _actionequip (Variables|Default|GetActionEquip))
  (bind _actionpickup (Variables|Default|GetActionPickUp))
  (bind _actionuse (Variables|Default|GetActionUse))
  (bind _verticalbox_2 (Variables|/Game/Blueprints/UI/WBP_BasicUI_v03.WBP_BasicUI_v03_C|GetVerticalBox_2 _wbp_hudv03))
  (bind _verticalbox_3 (Variables|/Game/Blueprints/UI/WBP_BasicUI_v03.WBP_BasicUI_v03_C|GetVerticalBox_3 _wbp_hudv03))
  (Widget|Panel|ClearChildren (Variables|/Game/Blueprints/UI/WBP_BasicUI_v03.WBP_BasicUI_v03_C|GetVerticalBox_3 (Variables|Default|GetWBP_HUDv03)))
  (Variables|Default|SetBoxIndex 0)
  (for _array_element (Variables|Default|GetWidgetArray)
    (if (>= (Class|PanelWidget|GetChildrenCount _verticalbox_2) 1)
      (Variables|Default|SetBoxIndex (+ (Variables|Default|GetBoxIndex) 1))
      (if (>= (Class|PanelWidget|GetChildrenCount _verticalbox_3) 3)
        (Variables|Default|SetBoxIndex (+ (Variables|Default|GetBoxIndex) 1))
        (Widget|Panel|AddChild (Variables|/Game/Blueprints/UI/WBP_BasicUI_v03.WBP_BasicUI_v03_C|GetVerticalBox_4 _wbp_hudv03) _array_element)
        (else
          (Widget|Panel|AddChild _verticalbox_3 _array_element)))
      (else
        (Widget|Panel|AddChild _verticalbox_2 _array_element))))
  (switch Utilities|FlowControl|Switch|SwitchonETTAction Selection
    (:Use
      (Widget|Panel|AddChild (CallFunction|GetVerticalBox) _actionuse)
      (Utilities|Array|AddUnique (Variables|Default|GetWidgetArray) _actionuse))
    (:Eat
      (Widget|Panel|AddChild (CallFunction|GetVerticalBox) _actioneat)
      (Utilities|Array|AddUnique (Variables|Default|GetWidgetArray) _actioneat))
    (:PickUp
      (Widget|Panel|AddChild (CallFunction|GetVerticalBox) _actionpickup)
      (Utilities|Array|AddUnique (Variables|Default|GetWidgetArray) _actionpickup))
    (:Drop
      (Widget|Panel|AddChild (CallFunction|GetVerticalBox) _actiondrop)
      (Utilities|Array|AddUnique (Variables|Default|GetWidgetArray) _actiondrop))
    (:Collect
      (Widget|Panel|AddChild (CallFunction|GetVerticalBox) _actioncollect)
      (Utilities|Array|AddUnique (Variables|Default|GetWidgetArray) _actioncollect))
    (:Craft
      (Widget|Panel|AddChild (CallFunction|GetVerticalBox) _actioncraft)
      (Utilities|Array|AddUnique (Variables|Default|GetWidgetArray) _actioncraft))
    (:Equip
      (Widget|Panel|AddChild (CallFunction|GetVerticalBox) _actionequip)
      (Utilities|Array|AddUnique (Variables|Default|GetWidgetArray) _actionequip))))

(fn RemoveActionCommand
  (params (Selection :type ETTAction%20Enum :default "Walk"))
  (bind _actioneat (Variables|Default|GetActionEat))
  (bind _actioncollect (Variables|Default|GetActionCollect))
  (bind _actioncraft (Variables|Default|GetActionCraft))
  (bind _actiondrop (Variables|Default|GetActionDrop))
  (bind _actionequip (Variables|Default|GetActionEquip))
  (bind _actionpickup (Variables|Default|GetActionPickUp))
  (bind _actionuse (Variables|Default|GetActionUse))
  (switch Utilities|FlowControl|Switch|SwitchonETTAction Selection
    (:Use
      (Widget|RemovefromParent _actionuse)
      (Utilities|Array|RemoveItem (Variables|Default|GetWidgetArray) _actionuse))
    (:Eat
      (Widget|RemovefromParent _actioneat)
      (Utilities|Array|RemoveItem (Variables|Default|GetWidgetArray) _actioneat))
    (:PickUp
      (Widget|RemovefromParent _actionpickup)
      (Utilities|Array|RemoveItem (Variables|Default|GetWidgetArray) _actionpickup))
    (:Drop
      (Widget|RemovefromParent _actiondrop)
      (Utilities|Array|RemoveItem (Variables|Default|GetWidgetArray) _actiondrop))
    (:Collect
      (Widget|RemovefromParent _actioncollect)
      (Utilities|Array|RemoveItem (Variables|Default|GetWidgetArray) _actioncollect))
    (:Craft
      (Widget|RemovefromParent _actioncraft)
      (Utilities|Array|RemoveItem (Variables|Default|GetWidgetArray) _actioncraft))
    (:Equip
      (Widget|RemovefromParent _actionequip)
      (Utilities|Array|RemoveItem (Variables|Default|GetWidgetArray) _actionequip)))
  (CallFunction|ManageVerticalBox))

(fn AddSubTaskTuturial
  (params (Class :type User%20Widget%20Class%20Reference))
  (bind _returnvalue (UserInterface|CreateWidget Class (Game|GetPlayerController 0)))
  (UserInterface|Viewport|AddtoViewport _returnvalue 0))

(fn GetVerticalBox
  (bind _wbp_hudv03 (Variables|Default|GetWBP_HUDv03))
  (return (Utilities|Select :Index (Variables|Default|GetBoxIndex) :Option%200 (Variables|/Game/Blueprints/UI/WBP_BasicUI_v03.WBP_BasicUI_v03_C|GetVerticalBox_2 _wbp_hudv03) :Option%201 (Variables|/Game/Blueprints/UI/WBP_BasicUI_v03.WBP_BasicUI_v03_C|GetVerticalBox_3 _wbp_hudv03) :Option%202 (Variables|/Game/Blueprints/UI/WBP_BasicUI_v03.WBP_BasicUI_v03_C|GetVerticalBox_4 _wbp_hudv03))))

(fn ManageVerticalBox
  (bind _wbp_hudv03 (Variables|Default|GetWBP_HUDv03))
  (bind _verticalbox_2 (Variables|/Game/Blueprints/UI/WBP_BasicUI_v03.WBP_BasicUI_v03_C|GetVerticalBox_2 _wbp_hudv03))
  (bind _verticalbox_3 (Variables|/Game/Blueprints/UI/WBP_BasicUI_v03.WBP_BasicUI_v03_C|GetVerticalBox_3 _wbp_hudv03))
  (Widget|Panel|ClearChildren (Variables|/Game/Blueprints/UI/WBP_BasicUI_v03.WBP_BasicUI_v03_C|GetVerticalBox_3 (Variables|Default|GetWBP_HUDv03)))
  (Variables|Default|SetBoxIndex 0)
  (for _array_element (Variables|Default|GetWidgetArray)
    (if (>= (Class|PanelWidget|GetChildrenCount _verticalbox_2) 1)
      (Variables|Default|SetBoxIndex (+ (Variables|Default|GetBoxIndex) 1))
      (if (>= (Class|PanelWidget|GetChildrenCount _verticalbox_3) 3)
        (Variables|Default|SetBoxIndex (+ (Variables|Default|GetBoxIndex) 1))
        (Widget|Panel|AddChild (Variables|/Game/Blueprints/UI/WBP_BasicUI_v03.WBP_BasicUI_v03_C|GetVerticalBox_4 _wbp_hudv03) _array_element)
        (else
          (Widget|Panel|AddChild _verticalbox_3 _array_element)))
      (else
        (Widget|Panel|AddChild _verticalbox_2 _array_element)))))